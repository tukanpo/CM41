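; Game board camera actor that frames a 2D board rectangle and plays an intro move toward it.
; It sets the camera pitch, then backs off from the rect center along the view axis by the distance ACCameraAutoFit calculates, so tilted views fit only approximately.
; The intro start sits 20% farther back.
; PlayInAnimation blends the view target to this actor, lerps location on a timeline, then calls OnInAnimationFinished.
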(event Custom|PlayInAnimation
  (params (StartLocation :type Vector) (TargetLocation :type Vector))
  (Development|PrintString "PlayInTransition Start")
  (Game|Player|SetViewTargetwithBlend (Game|GetPlayerController 0) self 0.0 "VTBlend_Cubic" 0.0 false)
  (bind _alpha (Timeline|InTransition Play)
    (:Update
      (Transformation|SetActorLocation (Math|Vector|Lerp(Vector) StartLocation TargetLocation _alpha) false false))
    (:Finished
      (Development|PrintString "PlayInAnimation Finished")
      (Default|CallOninAnimationFinished))))

(event EventBeginPlay)

(event Collision|EventActorBeginOverlap
  (params (OtherActor :type Actor%20Object%20Reference)))

(event EventTick
  (params (DeltaSeconds :type Float%20%28single-precision%29)))

(fn ConstructionScript)

(fn GetLocationtoFit2DRect
  (params (ViewTargetCenter :type Vector) (ViewTargetRect :type Vector%202D%20Structure) (Pitch :type Float%20%28double-precision%29))
  ;[0.15 0.15 0.15 0.5 16] カメラの角度を設定
  (Transformation|SetRelativeRotation (Variables|Default|GetCamera) (Math|Rotator|MakeRotator 0.0 Pitch 0.0) false false)
  (return (- ViewTargetCenter (* (Math|Vector|GetForwardVector (Variables|Default|GetCamera)) (Default|CalcCameraDistancetoFitRect (Variables|Default|GetAC_CameraAutoFit) (Variables|Default|GetCamera) ViewTargetRect)))))

(fn GetinAnimationLocations
  (params (ViewTargetCenter :type Vector) (ViewTargetRect :type Vector%202D%20Structure) (Pitch :type Float%20%28double-precision%29))
  (bind _output_get (LocalVariables|SetTargetLocation (CallFunction|GetLocationtoFit2DRect ViewTargetCenter ViewTargetRect Pitch)))
  (return (+ (LocalVariables|GetTargetLocation) (* (* (Math|Vector|GetForwardVector (Variables|Default|GetCamera)) -1.0) (* (Math|Vector|VectorLength (- (LocalVariables|GetTargetLocation) ViewTargetCenter)) 0.2))) _output_get))