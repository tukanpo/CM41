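; Unit command object for rotating a unit toward a new direction.
; SetParams stores the target unit and direction, then returns the command itself for chaining.
; Execute is currently empty: the logic that would pass the direction to the unit's rotate-state component and switch its state machine to that state is disconnected and never runs.
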(event EventExecute)

(fn SetParams
  (params (Unit :type BP%20Unit%20Object%20Reference) (NewDirection :type E_GridDirection%20Enum :default "NewEnumerator0"))
  (Variables|Default|SetUnit Unit)
  (Variables|Default|SetNewDirection NewDirection)
  (return self))