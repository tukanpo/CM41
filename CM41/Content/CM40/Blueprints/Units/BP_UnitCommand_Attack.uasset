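; BP_UnitCommand_Attack is a unit command intended to send a unit into its attack state.
; SetParams stores the unit, target cell index, direction and relative location, then returns the command itself.
; Execute is empty: the nodes that would pass those values to the attack state component and switch the unit's state machine to it are disconnected, so they never run.
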(event EventExecute)

(fn SetParams
  (params (Unit :type BP%20Unit%20Object%20Reference) (NewCellIndex :type Int%20Point%20Structure) (NewDirection :type E_GridDirection%20Enum :default "NewEnumerator0") (NewRelativeLocation :type Vector))
  (Variables|Default|SetUnit Unit)
  (Variables|Default|SetNewCellIndex NewCellIndex)
  (Variables|Default|SetNewDirection NewDirection)
  (Variables|Default|SetNewRelativeLocation NewRelativeLocation)
  (return self))