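; Unit state-machine state component that turns a unit to face a new direction.
; SetParams stores the target direction; EnterState writes it to the unit and starts a short timed rotation.
; When the rotation-finished event fires, it unbinds, signals that the unit action completed, then calls ChangeState with AC_UnitSM_RotateState, its own state name.
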(event Custom|EnterState_RotateToDirectionFinished
  (EventDispatchers|UnbindEventfromOnRotatetoDirectionFinished (Variables|Default|GetUnit) (delegate Custom|EnterState_RotateToDirectionFinished))
  ;[0.2396 0.2035 0 0.5 14] コメント
  (CallFunction|CallonUnitActionCompleted)
  ;[0.03665 0.3047 0 0.5 14] State 遷移
  (Default|ChangeState (Variables|Default|GetUnitSM) "AC_UnitSM_RotateState_C"))

(event EventBeginPlay
  (|CallParentFunction) ; このノードは無効になっているため呼び出せません。\n機能をビルドするにはピンをドラッグしてください。
)

(event EventTick
  (params (DeltaSeconds :type Float%20%28single-precision%29))
  (|CallParentFunction DeltaSeconds) ; このノードは無効になっているため呼び出せません。\n機能をビルドするにはピンをドラッグしてください。
)

(event EventEnterState
  (Variables|/Game/CM40/Blueprints/Units/BP_Unit.BP_Unit_C|SetDirection (Variables|Default|GetUnit) (Variables|Default|GetNewDirection))
  (EventDispatchers|BindEventtoOnRotatetoDirectionFinished (Variables|Default|GetUnit) (delegate Custom|EnterState_RotateToDirectionFinished))
  (Default|RotatetoDirection (Variables|Default|GetUnit) (Variables|Default|GetNewDirection) 0.2))

(fn SetParams
  (params (NewDirection :type E_GridDirection%20Enum :default "NewEnumerator0"))
  (Variables|Default|SetNewDirection NewDirection)
  (return))