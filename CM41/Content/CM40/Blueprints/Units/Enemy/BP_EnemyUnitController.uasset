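; Enemy unit controller for grid-based combat that decides the possessed BP_Unit's command.
; BeginPlay finds the level's BP_GameBoard and creates reusable move, rotate and attack command objects.
; DecideUnitCommand searches adjacent cells through CellUnitMap for any unit, without filtering for players, then configures, executes and returns an attack toward it.
; Move logic is unwired and the rotate command is unused.
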(event EventBeginPlay
  (Utilities|FlowControl|Sequence
    (:then_0
      ;[0.15 0.15 0.15 0.5 14] Level 上に GameBoard が配置済であること前提
      (bind _returnvalue (Actor|GetActorOfClass "/Game/CM40/Blueprints/GameBoard/BP_GameBoard.BP_GameBoard_C"))
      (Variables|Default|SetGameBoard _returnvalue))
    (:then_1
      ;[0.15 0.15 0.15 0.5 14] Command 生成
      (bind _returnvalue_2 (Game|ConstructObjectfromClass "/Game/CM40/Blueprints/Units/BP_UnitCommand_Move.BP_UnitCommand_Move_C"))
      (Variables|Default|SetUnitCommand_Move _returnvalue_2)
      (bind _returnvalue_3 (Game|ConstructObjectfromClass "/Game/CM40/Blueprints/Units/BP_UnitCommand_Rotate.BP_UnitCommand_Rotate_C"))
      (Variables|Default|SetUnitCommand_Rotate _returnvalue_3)
      (bind _returnvalue_4 (Game|ConstructObjectfromClass "/Game/CM40/Blueprints/Units/BP_UnitCommand_Attack.BP_UnitCommand_Attack_C"))
      (Variables|Default|SetUnitCommand_Attack _returnvalue_4))))

(event EventPossess
  (params (PossessedPawn :type Pawn%20Object%20Reference))
  (bind _asbp_unit (Utilities|Casting|CastToBP_Unit PossessedPawn))
  (Variables|Default|SetControlledUnit _asbp_unit))

(event EventUnPossess
  (params (UnpossessedPawn :type Pawn%20Object%20Reference))
  (Variables|Default|SetControlledUnit 0))

(fn ConstructionScript)

(fn DecideUnitCommand
  (params (CommandOuter :type Actor%20Object%20Reference))
  ;[0.15 0.15 0.15 0.5 14] この Unit の隣接セルに PlayerUnit が居るかチェック ＆ 取得
  (bind (_hitresult _hitcellindex) (CallFunction|FindAdjacentPlayerUnitCell (Variables|/Game/CM40/Blueprints/Units/BP_Unit.BP_Unit_C|GetCellIndex (Variables|Default|GetControlledUnit))))
  (if _hitresult
    (bind _newparam (CallFunction|CreateCommandAttack _hitcellindex))
    (return _newparam)))

(fn FindAdjacentPlayerUnitCell
  (params (CenterCellIndex :type Int%20Point%20Structure))
  (bind _result (Default|GetAdjacentCells (Variables|/Game/CM40/Blueprints/GameBoard/BP_GameBoard.BP_GameBoard_C|GetAC_Grid (Variables|Default|GetGameBoard)) CenterCellIndex))
  (bind _array_element (Utilities|Array|ForEachLoopwithBreak _result :!label _label)
    (:LoopBody
      (if (.ReturnValue (Utilities|Map|Find (Variables|/Game/CM40/Blueprints/GameBoard/BP_GameBoard.BP_GameBoard_C|GetCellUnitMap (Variables|Default|GetGameBoard)) _array_element))
        (LocalVariables|SetCellIndex (Variables|/Game/CM40/Blueprints/Units/BP_Unit.BP_Unit_C|GetCellIndex (.Value (Utilities|Map|Find (Variables|/Game/CM40/Blueprints/GameBoard/BP_GameBoard.BP_GameBoard_C|GetCellUnitMap (Variables|Default|GetGameBoard)) _array_element))))
        (LocalVariables|SetbHit true)
        (goto _label Break)))
    (:Completed
      (return (LocalVariables|GetbHit) (LocalVariables|GetCellIndex)))))

(fn CreateCommandAttack
  (params (ToCellIndex :type Int%20Point%20Structure))
  ;[0.15 0.15 0.15 0.5 14] プレイヤーへ攻撃する    （関数化）
  (bind _command (Default|SetParams (Variables|Default|GetUnitCommand_Attack) (Variables|Default|GetControlledUnit) ToCellIndex (Default|GetDirectionBetweenCells (Variables|/Game/CM40/Blueprints/GameBoard/BP_GameBoard.BP_GameBoard_C|GetAC_Grid (Variables|Default|GetGameBoard)) (Variables|/Game/CM40/Blueprints/Units/BP_Unit.BP_Unit_C|GetCellIndex (Variables|Default|GetControlledUnit)) ToCellIndex) (Default|GetCellRelativeLocation (Variables|/Game/CM40/Blueprints/GameBoard/BP_GameBoard.BP_GameBoard_C|GetAC_Grid (Variables|Default|GetGameBoard)) ToCellIndex)))
  (Default|Execute _command)
  (return (Variables|Default|GetUnitCommand_Attack)))