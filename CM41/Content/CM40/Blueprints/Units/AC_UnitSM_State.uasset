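; AC_UnitSM_State is a unit state machine state component, apparently a shared base for concrete unit states.
; On internal initialization it casts and caches the owning AC_UnitSM state machine and the BP_Unit owner.
; CallOnUnitActionCompleted reports back to the state machine through CallOnUnitActionFinished, passing the unit and always a false Result.
; BeginPlay and Tick are unused.
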(event EventBeginPlay
  (|CallParentFunction) ; このノードは無効になっているため呼び出せません。\n機能をビルドするにはピンをドラッグしてください。
)

(event EventTick
  (params (DeltaSeconds :type Float%20%28single-precision%29))
  (|CallParentFunction DeltaSeconds) ; このノードは無効になっているため呼び出せません。\n機能をビルドするにはピンをドラッグしてください。
)

(fn InitializeInternal
  (params (StateMachine :type AC%20State%20Machine%20Object%20Reference))
  (|CallParentFunction StateMachine)
  (Utilities|FlowControl|Sequence
    (:then_0
      (bind _asac_unit_sm (Utilities|Casting|CastToAC_UnitSM (Variables|Default|GetStateMachine)))
      (Variables|Default|SetUnitSM _asac_unit_sm))
    (:then_1
      (bind _asbp_unit (Utilities|Casting|CastToBP_Unit (Components|GetOwner)))
      (Variables|Default|SetUnit _asbp_unit))))

(fn CallonUnitActionCompleted
  (Default|CallOnUnitActionFinished (Variables|Default|GetUnitSM) (Variables|Default|GetUnit) false)
  (return))