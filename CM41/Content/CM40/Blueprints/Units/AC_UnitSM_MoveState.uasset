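; Unit state-machine state that performs a single move action for a unit.
; SetMoveParams stores the target cell index, direction and relative location.
; On enter, it rotates the unit to the new direction, spends one action point, then slides it to the new location, chaining the steps through bound finish events.
; When the move ends, it signals action completion and switches to the idle state.
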(event Custom|EnterState_RotateToDirectionFinished
  (EventDispatchers|UnbindEventfromOnRotatetoDirectionFinished (Variables|Default|GetUnit) (delegate Custom|EnterState_RotateToDirectionFinished))
  (Default|ModifyActionPoint (Variables|Default|GetUnit) -1)
  (EventDispatchers|BindEventtoOnSimpleMoveFinished (Variables|Default|GetUnit) (delegate Custom|EnterState_SimpleMoveFinished))
  (Default|SimpleMove (Variables|Default|GetUnit) (Variables|Default|GetNewRelativeLocation) 0.5))

(event Custom|EnterState_SimpleMoveFinished
  (EventDispatchers|UnbindEventfromOnSimpleMoveFinished (Variables|Default|GetUnit) (delegate Custom|EnterState_SimpleMoveFinished))
  ;[0.2396 0.2035 0 0.5] コメント
  (CallFunction|CallonUnitActionCompleted)
  ;[0.03665 0.3047 0 0.5 14] State 遷移
  (Default|ChangeState (Variables|Default|GetUnitSM) "/Game/CM40/Blueprints/Units/AC_UnitSM_IdleState.AC_UnitSM_IdleState_C"))

(event EventEnterState
  (Variables|/Game/CM40/Blueprints/Units/BP_Unit.BP_Unit_C|SetDirection (Variables|Default|GetUnit) (Variables|Default|GetNewDirection))
  (EventDispatchers|BindEventtoOnRotatetoDirectionFinished (Variables|Default|GetUnit) (delegate Custom|EnterState_RotateToDirectionFinished))
  (Default|RotatetoDirection (Variables|Default|GetUnit) (Variables|Default|GetNewDirection) 0.2))

(fn SetMoveParams
  (params (NewCellIndex :type Int%20Point%20Structure) (NewDirection :type E_GridDirection%20Enum :default "NewEnumerator0") (NewRelativeLocation :type Vector))
  (Variables|Default|SetNewCellIndex NewCellIndex)
  (Variables|Default|SetNewDirection NewDirection)
  (Variables|Default|SetNewRelativeLocation NewRelativeLocation)
  (return))