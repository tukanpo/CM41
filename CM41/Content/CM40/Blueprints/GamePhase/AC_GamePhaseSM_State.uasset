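; Base state component for the game phase state machine (AC_GamePhaseSM), owned by the GM_TestGame game mode.
; On internal initialization it calls the parent, then caches typed references to the state machine and game mode.
; From the game mode it also caches the game board, player unit, that unit's controller and the enemy unit manager.
; BeginPlay and Tick are disabled stubs; the file contains no phase logic of its own.
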(event EventBeginPlay
  (|CallParentFunction) ; このノードは無効になっているため呼び出せません。\n機能をビルドするにはピンをドラッグしてください。
)

(event EventTick
  (params (DeltaSeconds :type Float%20%28single-precision%29))
  (|CallParentFunction DeltaSeconds) ; このノードは無効になっているため呼び出せません。\n機能をビルドするにはピンをドラッグしてください。
)

(fn InitializeInternal
  (params (StateMachine :type AC%20State%20Machine%20Object%20Reference))
  (|CallParentFunction StateMachine)
  (Utilities|FlowControl|Sequence
    (:then_0
      (bind _asac_game_phase_sm (Utilities|Casting|CastToAC_GamePhaseSM (Variables|Default|GetStateMachine)))
      (Variables|Default|SetGamePhase2SM _asac_game_phase_sm))
    (:then_1
      (bind _asgm_test_game (Utilities|Casting|CastToGM_TestGame (Components|GetOwner)))
      (Variables|Default|SetTestGame2 _asgm_test_game)
      (Variables|Default|SetGameBoard (Variables|/Game/CM40/Blueprints/GM_TestGame.GM_TestGame_C|GetGameBoard (Variables|Default|GetTestGame2))))
    (:then_2
      (Variables|Default|SetPlayerUnit (Variables|/Game/CM40/Blueprints/GM_TestGame.GM_TestGame_C|GetPlayerUnit (Variables|Default|GetTestGame2)))
      (bind _asbp_player_unit_controller (Utilities|Casting|CastToBP_PlayerUnitController (Pawn|GetController (Variables|Default|GetPlayerUnit))))
      (Variables|Default|SetPlayerUnitController _asbp_player_unit_controller)
      (Variables|Default|SetEnemyUnitManager (Variables|/Game/CM40/Blueprints/GM_TestGame.GM_TestGame_C|GetEnemyUnitManager (Variables|Default|GetTestGame2))))))