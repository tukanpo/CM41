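; AC_ActorPool is an actor component that pools reusable actors by class, for classes implementing the BI_Activatable interface.
; AddPool validates the class, stores pool data in the Pools map and pre-spawns the initial count through AddActor, which deactivates each new actor.
; GetActorFromPool returns the first inactive actor, spawning another when none is free, and leaves activation to the caller.
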(event EventBeginPlay)

(event EventTick
  (params (DeltaSeconds :type Float%20%28single-precision%29)))

(fn AddPool
  (params (TargetClass :type Actor%20Class%20Reference) (InitialPoolSize :type Integer))
  ;[0.15 0.15 0.15 0.5 14] 対象クラスのインターフェース実装チェック
  (if (Class|KismetSystemLibrary|DoesClassImplementInterface TargetClass "/Game/CM40/Blueprints/Common/BI_Activatable.BI_Activatable_C")
    ;[0.15 0.15 0.15 0.5 14] プール重複チェック
    (if (not (Utilities|Map|Contains (Variables|Default|GetPools) TargetClass))
      ;[0.15 0.15 0.15 0.5 14] プール追加
      (Utilities|Map|Add (Variables|Default|GetPools) TargetClass (Utilities|Struct|MakeF_ActorPoolData TargetClass 0 InitialPoolSize))
      ;[0.15 0.15 0.15 0.5 14] 初期プールサイズの分だけ Actor を生成する。
      (for _index (range 0 (- InitialPoolSize 1))
        (CallFunction|AddActor TargetClass))
      (return)
      (else
        (Development|PrintString "AddPool: Already Exists" true true "(R=0.239583,G=0.035563,B=0.053270,A=0.500000)" 1e+02)))
    (else
      (Development|PrintString "AddPool: Does Not BI_Activatable interface" true true "(R=0.239583,G=0.035563,B=0.053270,A=0.500000)" 1e+02)))
  (return))

(fn AddActor
  (params (TargetClass :type Actor%20Class%20Reference))
  (bind _returnvalue (Game|SpawnActorfromClass TargetClass (Math|Transform|MakeTransform "0, 0, 0" "0, 0, 0" "1.000000,1.000000,1.000000") "AlwaysSpawn" "MultiplyWithRoot" 0 0))
  (bind _asbi_activatable (Utilities|Casting|CastToBI_Activatable _returnvalue))
  (bind _output_get (LocalVariables|SetLocalPoolData (.Value (Utilities|Map|Find (Variables|Default|GetPools) TargetClass))))
  (Utilities|Array|AddUnique (.pooledobjects _output_get) _asbi_activatable)
  (Utilities|Map|Add (Variables|Default|GetPools) TargetClass (LocalVariables|GetLocalPoolData))
  (Default|Deactive _asbi_activatable) ; 初期状態は Inactive
  (return _asbi_activatable))

(fn GetActorfromPool
  (params (TargetClass :type Actor%20Class%20Reference))
  ;[0.15 0.15 0.15 0.5 14] プールから Inactive オブジェクトを取得
  (bind _array_element (Utilities|Array|ForEachLoopwithBreak (.pooledobjects (.Value (Utilities|Map|Find (Variables|Default|GetPools) TargetClass))) :!label _label)
    (:LoopBody
      (bind _actor (Utilities|IsActiveMacro _array_element)
        (:true
          (LocalVariables|SetHitElement _actor)
          (goto _label Break))))
    (:Completed
      (Utilities|IsValid (Utilities|ToObject(Interface) (LocalVariables|GetHitElement))
        (:Is%20Valid
          _)
        (:Is%20Not%20Valid
          ;[0.15 0.15 0.15 0.5 14] 無ければプールに追加
          (bind _result (CallFunction|AddActor TargetClass))
          (LocalVariables|SetHitElement _result)))
      (return (LocalVariables|GetHitElement)))))