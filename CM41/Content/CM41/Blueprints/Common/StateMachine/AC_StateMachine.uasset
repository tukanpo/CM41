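; AC_StateMachine is an actor component that runs a class-keyed state machine over AC_State components on its owner.
; Initialization gathers owner components of a given class into a map and links each back to the machine.
; State changes ask the current state for permission, then wait for its exit-finished event before entering the next, allowing asynchronous exits.
; The first change skips exit, and missing states print an error.
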(event Custom|ProcessChangeState
  (params (NextState :type AC%20State%20Class%20Reference))
  ;[0.15 0.15 0.15 0.5 14] 初回ならExitをスキップ
  (Utilities|IsValid (Variables|Default|GetCurrentState)
    (:Is%20Valid
      (EventDispatchers|BindEventtoOnExitStateFinished (Variables|Default|GetCurrentState) (delegate Custom|ChangeState_OnExitStateFinished))
      (Default|ExitState (Variables|Default|GetCurrentState)))
    (:Is%20Not%20Valid
      (bind _output_get (Variables|Default|SetCurrentState (.Value (Utilities|Map|Find (Variables|Default|GetStates) NextState))))
      (Utilities|IsValid _output_get
        (:Is%20Valid
          (Development|PrintString (Utilities|GetDisplayName _output_get))
          (Default|CallOnStateChanged)
          (Default|EnterState (Variables|Default|GetCurrentState)))
        (:Is%20Not%20Valid
          ;[0.2396 0.2035 0 0.5 14] 次の State が StateMachine に存在しない時のエラー出力
          (Development|PrintString (Utilities|String|BuildString(Name) "State Not Found!  " "[" (Utilities|String|StringToName (Utilities|GetClassDisplayName NextState)) "]") true true "(R=0.239583,G=0.035563,B=0.053270,A=0.500000)" 1e+02))))))

(event Custom|ChangeState_OnExitStateFinished
  (EventDispatchers|UnbindEventfromOnExitStateFinished (Variables|Default|GetCurrentState) (delegate Custom|ChangeState_OnExitStateFinished))
  (bind _output_get (Variables|Default|SetCurrentState (.Value (Utilities|Map|Find (Variables|Default|GetStates) (stale Custom|ProcessChangeState NextState)))))
  (Utilities|IsValid _output_get
    (:Is%20Valid
      (Development|PrintString (Utilities|GetDisplayName _output_get))
      (Default|CallOnStateChanged)
      (Default|EnterState (Variables|Default|GetCurrentState)))
    (:Is%20Not%20Valid
      ;[0.2396 0.2035 0 0.5 14] 次の State が StateMachine に存在しない時のエラー出力
      (Development|PrintString (Utilities|String|BuildString(Name) "State Not Found!  " "[" (Utilities|String|StringToName (Utilities|GetClassDisplayName (stale Custom|ProcessChangeState NextState))) "]") true true "(R=0.239583,G=0.035563,B=0.053270,A=0.500000)" 1e+02))))

(event EventBeginPlay)

(event EventTick
  (params (DeltaSeconds :type Float%20%28single-precision%29)))

(fn InitializeInternal
  (params (StateClass :type AC%20State%20Class%20Reference))
  ;[0.15 0.15 0.15 0.5 14] Owner にアタッチされている同一タイプの AC_State コンポーネントを全てリストに追加する
  (for _array_element (Actor|GetComponentsByClass (Components|GetOwner) StateClass)
    (CallFunction|AddStateInternal _array_element))
  (return))

(fn AddStateInternal
  (params (State :type AC%20State%20Object%20Reference))
  (Default|InitializeInternal State self)
  (Utilities|Map|Add (Variables|Default|GetStates) (Utilities|GetClass State) State)
  (return))

(fn ChangeStateInternal
  (params (NewState :type AC%20State%20Class%20Reference))
  ;[0.15 0.15 0.15 0.5] コメント
  (Utilities|IsValid (Variables|Default|GetCurrentState)
    (:Is%20Valid
      (bind _newparam (Default|CanChangeState (Variables|Default|GetCurrentState)))
      (if _newparam
        (CallFunction|ProcessChangeState NewState))
      (return _newparam))
    (:Is%20Not%20Valid
      (CallFunction|ProcessChangeState NewState)
      (return true))))