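; Grid component that stores a map of cells and provides coordinate, bounds, direction and four-way neighbour queries.
; Initialize builds the cells and N/S/E/W lookup maps from grid size and cell size.
; Conversions use the component's transform and swap X/Y, so grid Y follows Unreal X, with cell origins at cell centres.
; GetAdjacentCells uses GetCellOffsetByDirection, whose X/Y offsets are transposed relative to DirectionToCellIndexMap.
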(event EventBeginPlay)

(event EventTick
  (params (DeltaSeconds :type Float%20%28single-precision%29)))

(fn Initialize
  (params (GridSizeX :type Integer) (GridSizeY :type Integer) (CellSize :type Float%20%28double-precision%29))
  (Development|PrintString "Initialize")
  (Utilities|FlowControl|Sequence
    (:then_0
      (Variables|Default|SetGridSizeX GridSizeX)
      (Variables|Default|SetGridSizeY GridSizeY)
      (Variables|Default|SetCellSize CellSize))
    (:then_1
      (Private|MakeDeltaCellIndextoDirectionMap)
      (Private|MakeDirectiontoCellIndexMap)
      (Private|MakeDirectiontoWorldVectorMap))
    (:then_2
      (Utilities|Map|Clear (Variables|Default|GetCells))
      (for _index (range 0 (- (Variables|Default|GetGridSizeX) 1)) ; Xループ
        (LocalVariables|SetCurrentX _index)
        (for _index_2 (range 0 (- GridSizeY 1)) ; Yループ
          (LocalVariables|SetCurrentY _index_2)
          (Utilities|Map|Add (Variables|Default|GetCells) (Utilities|Struct|MakeIntPoint (LocalVariables|GetCurrentX) (LocalVariables|GetCurrentY)) (Utilities|Struct|MakeF_GridCell (LocalVariables|GetCurrentX) (LocalVariables|GetCurrentY)))))
      (return))))

(fn MakeDeltaCellIndextoDirectionMap
  (Utilities|Map|Clear (Variables|Default|GetDeltaCellIndexToDirectionMap))
  (Utilities|Map|Add (Variables|Default|GetDeltaCellIndexToDirectionMap) (Utilities|Struct|MakeIntPoint 0 1) "NewEnumerator0")
  (Utilities|Map|Add (Variables|Default|GetDeltaCellIndexToDirectionMap) (Utilities|Struct|MakeIntPoint 0 -1) "NewEnumerator1")
  (Utilities|Map|Add (Variables|Default|GetDeltaCellIndexToDirectionMap) (Utilities|Struct|MakeIntPoint 1 0) "NewEnumerator2")
  (Utilities|Map|Add (Variables|Default|GetDeltaCellIndexToDirectionMap) (Utilities|Struct|MakeIntPoint -1 0) "NewEnumerator3")
  (return))

(fn MakeDirectiontoCellIndexMap
  (Utilities|Map|Clear (Variables|Default|GetDirectionToCellIndexMap))
  (Utilities|Map|Add (Variables|Default|GetDirectionToCellIndexMap) "NewEnumerator0" (Utilities|Struct|MakeIntPoint 0 1))
  (Utilities|Map|Add (Variables|Default|GetDirectionToCellIndexMap) "NewEnumerator1" (Utilities|Struct|MakeIntPoint 0 -1))
  (Utilities|Map|Add (Variables|Default|GetDirectionToCellIndexMap) "NewEnumerator2" (Utilities|Struct|MakeIntPoint 1 0))
  (Utilities|Map|Add (Variables|Default|GetDirectionToCellIndexMap) "NewEnumerator3" (Utilities|Struct|MakeIntPoint -1 0))
  (return))

(fn MakeDirectiontoWorldVectorMap
  (Utilities|Map|Clear (Variables|Default|GetDirectionToWorldVectorMap))
  (Utilities|Map|Add (Variables|Default|GetDirectionToWorldVectorMap) "NewEnumerator0" "1.000000,0.000000,0.000000")
  (Utilities|Map|Add (Variables|Default|GetDirectionToWorldVectorMap) "NewEnumerator1" "-1.000000,0.000000,0.000000")
  (Utilities|Map|Add (Variables|Default|GetDirectionToWorldVectorMap) "NewEnumerator2" "0.000000,1.000000,0.000000")
  (Utilities|Map|Add (Variables|Default|GetDirectionToWorldVectorMap) "NewEnumerator3" "0.000000,-1.000000,0.000000")
  (return))

(fn GetCell
  (params (CellIndex :type Int%20Point%20Structure))
  (return (.Value (Utilities|Map|Find (Variables|Default|GetCells) CellIndex))))

(fn GetGridWorldSize
  (return (Math|Vector2D|MakeVector2D (* (Variables|Default|GetGridSizeX) (Variables|Default|GetCellSize)) (* (Variables|Default|GetGridSizeY) (Variables|Default|GetCellSize)))))

(fn GetGridWorldCenter
  (return (+ (Transformation|GetWorldLocation) (Math|Vector|MakeVector (* (* (- (Variables|Default|GetGridSizeY) 1) (Variables|Default|GetCellSize)) 0.5) (* (* (- (Variables|Default|GetGridSizeX) 1) (Variables|Default|GetCellSize)) 0.5) 0.0))))

(fn GetCellRelativeLocation
  (params (CellIndex :type Int%20Point%20Structure))
  (bind (_x _y) (Utilities|Struct|BreakIntPoint CellIndex))
  (bind _cellsize (Variables|Default|GetCellSize))
  (return (Math|Vector|MakeVector (* _y _cellsize) (* _x _cellsize) 0.0)))

(fn GetCellWorldLocation
  (params (CellIndex :type Int%20Point%20Structure))
  (return (Math|Transform|TransformLocation (Transformation|GetWorldTransform) (CallFunction|GetCellRelativeLocation CellIndex))))

(fn WorldLocationtoCellIndex
  (params (WorldLocation :type Vector))
  (bind _returnvalue (Transformation|GetWorldTransform))
  (bind _cellsize (Variables|Default|GetCellSize))
  (bind _returnvalue_2 (Math|Transform|InverseTransformLocation _returnvalue WorldLocation))
  (return (Utilities|Struct|MakeIntPoint (Math|Float|Floor (/ (.y _returnvalue_2) _cellsize)) (Math|Float|Floor (/ (.x _returnvalue_2) _cellsize)))))

(fn IsinGridBounds
  (params (CellIndex :type Int%20Point%20Structure))
  (bind (_x _y) (Utilities|Struct|BreakIntPoint CellIndex))
  (return (and (and (>= _x 0) (< _x (Variables|Default|GetGridSizeX))) (and (>= _y 0) (< _y (Variables|Default|GetGridSizeY))))))

(fn GetDirectionBetweenCells
  (params (FromCellIndex :type Int%20Point%20Structure) (ToCellIndex :type Int%20Point%20Structure))
  (bind _direction (CallFunction|GetDirectionbyDeltaIndex (- ToCellIndex FromCellIndex)))
  (return _direction))

(fn GetDirectionbyDeltaIndex
  (params (DeltaIndex :type Int%20Point%20Structure))
  (LocalVariables|SetDeltaX (.x DeltaIndex))
  (LocalVariables|SetDeltaY (.y DeltaIndex))
  (if (> (Math|Integer|Absolute(Integer) (LocalVariables|GetDeltaX)) (Math|Integer|Absolute(Integer) (LocalVariables|GetDeltaY)))
    (if (> (LocalVariables|GetDeltaX) 0)
      (return "NewEnumerator2")
      (else
        (return "NewEnumerator3")))
    (elif (> (LocalVariables|GetDeltaY) 0)
      (return "NewEnumerator0")
      (else
        (return "NewEnumerator1")))))

(fn DirectiontoCellOffset
  (params (Direction :type E_GridDirection%20Enum :default "NewEnumerator0"))
  (return (.Value (Utilities|Map|Find (Variables|Default|GetDirectionToCellIndexMap) Direction))))

(fn GetCellOffsetbyDirection
  (params (Direction :type E_GridDirection%20Enum :default "NewEnumerator0"))
  (switch Utilities|FlowControl|Switch|SwitchonE_GridDirection Direction
    (:NewEnumerator0
      (return (Utilities|Struct|MakeIntPoint 1 0)))
    (:NewEnumerator1
      (return (Utilities|Struct|MakeIntPoint -1 0)))
    (:NewEnumerator2
      (return (Utilities|Struct|MakeIntPoint 0 1)))
    (:NewEnumerator3
      (return (Utilities|Struct|MakeIntPoint 0 -1)))))

(fn GetAdjacentCells
  (params (CenterCellIndex :type Int%20Point%20Structure))
  (bind _enumvalue (|ForEachE_GridDirection)
    (:LoopBody
      (bind _result (CallFunction|GetCellOffsetbyDirection _enumvalue))
      (bind _output_get (LocalVariables|SetWorkCellIndex (+ _result CenterCellIndex)))
      (if (CallFunction|IsinGridBounds _output_get)
        (Utilities|Array|AddUnique (LocalVariables|GetWorkCells) (LocalVariables|GetWorkCellIndex))))
    (:then
      (return (LocalVariables|GetWorkCells)))))