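; Camera helper component that calculates how far a camera must be to fit a rectangle in the viewport.
; CalcCameraDistanceToFitRect compares rectangle and viewport aspect ratios, then divides width or height by the matching half-FOV tangent.
; The height branch treats the camera's FieldOfView as vertical.
; The width branch derives horizontal FOV from the aspect ratio but passes zero as vertical FOV, so its tangent evaluates to zero.
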(event EventBeginPlay)

(event EventTick
  (params (DeltaSeconds :type Float%20%28single-precision%29)))

(fn GetHalfVFovTan
  (params (VFov :type Float%20%28double-precision%29))
  (return (Math|Trig|Tan(Radians) (Math|Trig|DegreesToRadians (* VFov 0.5)))))

(fn GetHalfHFovTan
  (params (ViewportAspectRatio :type Float%20%28double-precision%29))
  (return (Math|Trig|Tan(Radians) (Math|Trig|Atan(Degrees) (* ViewportAspectRatio (CallFunction|GetHalfVFovTan 0.0))))))

(fn CalcCameraDistancetoFitRect
  (params (Camera :type Camera%20Component%20Object%20Reference) (Rect :type Vector%202D%20Structure))
  (bind _returnvalue (Viewport|GetViewportSize))
  (LocalVariables|SetRectX (.x Rect))
  (LocalVariables|SetRectY (.y Rect))
  (Utilities|FlowControl|Sequence
    (:then_0
      (LocalVariables|SetRectAspectRatio (/ (LocalVariables|GetRectX) (LocalVariables|GetRectY))))
    (:then_1
      (LocalVariables|SetViewportAspectRatio (/ (.x _returnvalue) (.y _returnvalue))))
    (:then_2
      (if (> (LocalVariables|GetRectAspectRatio) (LocalVariables|GetViewportAspectRatio))
        (return (/ (LocalVariables|GetRectX) (CallFunction|GetHalfHFovTan (LocalVariables|GetViewportAspectRatio))))
        (else
          (return (/ (LocalVariables|GetRectY) (CallFunction|GetHalfVFovTan (Variables|/Script/Engine.CameraComponent|GetFieldOfView Camera)))))))))