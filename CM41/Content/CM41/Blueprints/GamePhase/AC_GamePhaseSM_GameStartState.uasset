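; Game phase state machine state that runs game start: board setup, player spawn, then handoff to the turn loop.
; On enter it initializes a 4x4 GameBoard with default tiles, then places and activates the PlayerUnit on a random free cell with random facing, in idle state.
; Bind-then-unbind delegates chain spawn completion into the board's intro animation, whose completion switches to TurnLoopStartState.
; With no free cell it only prints an error, stalling the phase.
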(event Custom|EnterState_InAnimationFInished
  ;[0.15 0.15 0.15 0.5 14] GameBoard の In アニメーションを実行して待機
  (EventDispatchers|UnbindEventfromOninAnimationFinished (Variables|Default|GetGameBoard) (delegate Custom|EnterState_InAnimationFInished))
  ;[0.03665 0.3047 0 0.5 14] 次ステートへ遷移
  (Default|ChangeState (Variables|Default|GetGamePhase2SM) "/Game/CM41/Blueprints/GamePhase/AC_GamePhaseSM_TurnLoopStartState.AC_GamePhaseSM_TurnLoopStartState_C"))

(event Custom|SpawnPlayerRandomCell
  ;[0.15 0.15 0.15 0.5 14] Grid 上のランダムな Cell にプレイヤーを配置してアクティブ化  (Spawn 演出を後で入れる)
  (bind (_cellindex _result) (Default|GetRandomFreeCell (Variables|Default|GetGameBoard)))
  (if _result
    (Default|PlaceUnitonCell (Variables|Default|GetGameBoard) (Variables|Default|GetPlayerUnit) _cellindex (Default|GetRandomDirection (Variables|Default|GetGameBoard)))
    (Default|Activate (Variables|Default|GetPlayerUnit))
    (Default|ChangeState (Variables|/Game/CM41/Blueprints/Units/BP_Unit.BP_Unit_C|GetAC_UnitSM (Variables|Default|GetPlayerUnit)) "/Game/CM41/Blueprints/Units/AC_UnitSM_IdleState.AC_UnitSM_IdleState_C")
    (Default|CallOnSpawnPlayerFinished)
    (else
      (Development|PrintString "SpawnPlayerRandomCell : No Free Cell!" true true "(R=1.000000,G=0.000000,B=0.000000,A=1.000000)" 1e+02))))

(event Custom|EnterState_SpawnPlayerFinished
  ;[0.15 0.15 0.15 0.5 14] PlayerUnit を GameBoard 上に配置
  (EventDispatchers|UnbindEventfromOnSpawnPlayerFinished (delegate Custom|EnterState_SpawnPlayerFinished))
  ;[0.15 0.15 0.15 0.5 14] GameBoard の In アニメーションを実行して待機
  (EventDispatchers|BindEventtoOninAnimationFinished (Variables|Default|GetGameBoard) (delegate Custom|EnterState_InAnimationFInished))
  (Default|PlayinAnimation (Variables|Default|GetGameBoard)))

(event EventEnterState
  ;[0.15 0.15 0.15 0.5 14] GameBoard 初期化
  ;;[0.2396 0.2035 0 0.5 14] GridSize の可変化はどうするか？
  (Default|Initialize (Variables|Default|GetGameBoard) (Utilities|Struct|MakeIntPoint 4 4) (Variables|/Game/CM41/Blueprints/GameBoard/BP_GameBoard.BP_GameBoard_C|GetCellSize (Variables|Default|GetGameBoard)) true)
  ;[0.15 0.15 0.15 0.5 14] PlayerUnit を GameBoard 上に配置
  (EventDispatchers|BindEventtoOnSpawnPlayerFinished (delegate Custom|EnterState_SpawnPlayerFinished))
  (CallFunction|SpawnPlayerRandomCell))