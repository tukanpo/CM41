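; Game phase state machine state that runs the enemies' turn.
; On entry it has EnemyUnitManager decide commands for the spawned enemy units, binds to the all-commands-finished event, then executes the commands and waits.
; When every enemy command finishes, it unbinds and switches GamePhase2SM to the turn loop start state.
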(event Custom|EnterState_AllEnemyCommandsFinished
  ;[0.15 0.15 0.15 0.5 14] すべての敵の Command を実行し、完了を待つ
  (EventDispatchers|UnbindEventfromOnAllEnemyCommandsFinished (Variables|Default|GetEnemyUnitManager) (delegate Custom|EnterState_AllEnemyCommandsFinished))
  ;[0.03665 0.3047 0 0.5 14] 次ステートへ遷移
  (Default|ChangeState (Variables|Default|GetGamePhase2SM) "/Game/CM41/Blueprints/GamePhase/AC_GamePhaseSM_TurnLoopStartState.AC_GamePhaseSM_TurnLoopStartState_C"))

(event EventEnterState
  ;[0.2396 0.2035 0 0.5 14] スポーン済の敵のCommand決定
  (Default|DecideUnitCommands (Variables|Default|GetEnemyUnitManager))
  ;[0.15 0.15 0.15 0.5 14] すべての敵の Command を実行し、完了を待つ
  (EventDispatchers|BindEventtoOnAllEnemyCommandsFinished (Variables|Default|GetEnemyUnitManager) (delegate Custom|EnterState_AllEnemyCommandsFinished))
  (Default|ExecuteandWaitCommands (Variables|Default|GetEnemyUnitManager)))