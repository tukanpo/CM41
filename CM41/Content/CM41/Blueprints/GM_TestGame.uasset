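; GM_TestGame is a game mode that sets up the board and units, then starts the game-phase flow.
; After a short delay to let placed actors finish BeginPlay, it caches the level's BP_GameBoard and the player pawn as BP_PlayerUnit.
; It spawns a BP_EnemyUnitManager initialized with the board.
; It then initializes the component-based GamePhase state machine and enters its GameStart state.
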(event EventBeginPlay
  ;[0.2396 0.2035 0 0.5 14] レベル上に配置された Actor の BeginPlay を待ってから開始する
  (Utilities|FlowControl|Delay 0.2)
  (Utilities|FlowControl|Sequence
    (:then_0
      ;[0.15 0.15 0.15 0.5 14] レベル上にある Actor の参照取得や生成を行う
      (CallFunction|Initialize))
    (:then_2
      ;[0.15 0.15 0.15 0.5 14] GamePhase ステートマシンの初期化と実行
      (Default|Initialize (Variables|Default|GetAC_GamePhaseSM) "/Game/CM41/Blueprints/GamePhase/AC_GamePhaseSM_State.AC_GamePhaseSM_State_C")
      (Default|ChangeState (Variables|Default|GetAC_GamePhaseSM) "/Game/CM41/Blueprints/GamePhase/AC_GamePhaseSM_GameStartState.AC_GamePhaseSM_GameStartState_C"))))

(fn ConstructionScript)

(fn Initialize
  (Utilities|FlowControl|Sequence
    (:then_0
      ;[0.15 0.15 0.15 0.5 14] レベルに配置されている BP_GameBoard を取得して保持
      (bind _returnvalue (Actor|GetActorOfClass "/Game/CM41/Blueprints/GameBoard/BP_GameBoard.BP_GameBoard_C"))
      (bind _output_get (Variables|Default|SetGameBoard _returnvalue))
      (Utilities|IsValid _output_get
        (:Is%20Not%20Valid
          (Development|PrintString "レベル上にGameBoardが無い！" true true "(R=0.239583,G=0.035563,B=0.053270,A=1.000000)" 1e+03))))
    (:then_1
      ;[0.15 0.15 0.15 0.5 14] PlayerUnit （ワールドセッティングで設定済の想定）
      (bind _asbp_player_unit (Utilities|Casting|CastToBP_PlayerUnit (Game|Player|GetPlayerPawn 0)))
      (Variables|Default|SetPlayerUnit _asbp_player_unit))
    (:then_2
      ;[0.15 0.15 0.15 0.5 14] 敵のマネージャークラス
      (bind _returnvalue_2 (Game|SpawnActorfromClass "/Game/CM41/Blueprints/Units/Enemy/BP_EnemyUnitManager.BP_EnemyUnitManager_C" (Math|Transform|MakeTransform "0, 0, 0" "0, 0, 0" "1.000000,1.000000,1.000000") "Undefined" "MultiplyWithRoot" 0 0))
      (bind _output_get_2 (Variables|Default|SetEnemyUnitManager _returnvalue_2))
      (Default|Initialize _output_get_2 (Variables|Default|GetGameBoard)))))