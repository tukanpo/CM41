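; AC_UnitSM_HitReactionState is the unit state machine state that runs a unit's hit reaction.
; On entering, it binds to the Unit's hit-reaction-finished event and starts the reaction.
; When that event fires, it unbinds, signals that the unit action has finished and switches UnitSM to the idle state.
; SetParams stores a NewDirection, which the state's event graph does not read.
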(event Custom|EnterState_HitReactionFinished
  (EventDispatchers|UnbindEventfromOnHitReactionFinished (Variables|Default|GetUnit) (delegate Custom|EnterState_HitReactionFinished))
  (CallFunction|CallonUnitActionFinished)
  ;[0.03665 0.3047 0 0.5 14] State 遷移
  (Default|ChangeState (Variables|Default|GetUnitSM) "/Game/CM41/Blueprints/Units/AC_UnitSM_IdleState.AC_UnitSM_IdleState_C"))

(event EventEnterState
  (EventDispatchers|BindEventtoOnHitReactionFinished (Variables|Default|GetUnit) (delegate Custom|EnterState_HitReactionFinished))
  (Default|PlayHitReaction (Variables|Default|GetUnit)))

(fn SetParams
  (params (NewDirection :type E_GridDirection%20Enum :default "NewEnumerator0"))
  (Variables|Default|SetNewDirection NewDirection)
  (return))