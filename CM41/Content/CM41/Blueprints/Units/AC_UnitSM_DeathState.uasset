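; Unit state machine component for the death state, which runs a unit's death and reports when it finishes.
; On entry it binds to the unit's OnDeathFinished event, then calls Death on the unit.
; When that event fires, it unbinds and passes the unit to its controller through HandleDeathFinishedMessage.
; SetParams stores a direction that the death logic in this graph never reads.
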(event Custom|EnterState_DeathFinished
  (EventDispatchers|UnbindEventfromOnDeathFinished (Variables|Default|GetUnit) (delegate Custom|EnterState_DeathFinished))
  (Class|BPIUnitEventHandler|HandleDeathFinished(Message) (Pawn|GetController (Variables|Default|GetUnit)) (Variables|Default|GetUnit)))

(event EventEnterState
  (EventDispatchers|BindEventtoOnDeathFinished (Variables|Default|GetUnit) (delegate Custom|EnterState_DeathFinished))
  (Default|Death (Variables|Default|GetUnit)))

(fn SetParams
  (params (NewDirection :type E_GridDirection%20Enum :default "NewEnumerator0"))
  (Variables|Default|SetNewDirection NewDirection)
  (return))