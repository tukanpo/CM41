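; BP_EnemyUnitManager spawns enemy units on the game board and runs their commands.
; When no living enemies remain, it spawns a pack from an actor pool onto random free cells with random facing, counting down to signal pack completion.
; It asks each standby unit's BP_EnemyUnitController for a command, then executes the collected commands in order.
; Units marked dead are removed in bulk before each pack spawn check.
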(event Custom|SpawnEnemyUnit
  (params (EnemyUnit :type BP%20Unit%20Object%20Reference))
  (bind _unit (CallFunction|PlaceUnitonRandomFreeCell EnemyUnit))
  (Default|Activate _unit)
  ;[0.15 0.15 0.15 0.5 14] 待機ユニット配列に入れる
  (Utilities|Array|AddUnique (Variables|Default|GetActiveEnemyUnits) (Utilities|Struct|MakeF_EnemyUnitData _unit true false))
  (Default|CallOnSpawnEnemyUnitFinished))

(event Custom|SpawnEnemyPack
  (params (SpawnCount :type Integer))
  ;[0.15 0.15 0.15 0.5 14] 死亡をマークされた敵を配列から一括削除する
  (CallFunction|RemoveDeadUnits)
  ;[0.15 0.15 0.15 0.5 14] 敵ユニット数が０なら次のパックをスポーンする
  (if (and (== (Utilities|Array|Length (Variables|Default|GetActiveEnemyUnits)) 0) (> SpawnCount 0))
    (bind _output_get (Variables|Default|SetRemainingSpawnCount SpawnCount))
    (bind _output_get_2 (Variables|Default|SetSpawnLoopIndexMax (- _output_get 1)))
    (for _index (range 0 _output_get_2)
      (bind _result (Default|GetActorfromPool (Variables|Default|GetAC_ActorPool) "/Game/CM41/Blueprints/Units/Enemy/BP_EnemyUnit.BP_EnemyUnit_C"))
      (bind _asbp_unit (Utilities|Casting|CastToBP_Unit _result))
      (CallFunction|SpawnEnemyUnit _asbp_unit))
    (else
      (Default|CallOnSpawnEnemyPackFinished))))

(event Custom|ExecuteAndWaitCommands
  (for _array_element (Variables|Default|GetUnitCommands)
    (Default|Execute _array_element)))

(event Custom|BeginPlay_SpawnEnemyUnitFinished
  ;[0.15 0.15 0.15 0.5 14] すべての敵をスポーンさせたら完了通知を送る
  (bind _result (Math|Integer|DecrementInt (Variables|Default|GetRemainingSpawnCount))
    (:%20%20
      (if (<= _result 0)
        (Default|CallOnSpawnEnemyPackFinished)))))

(event EventBeginPlay
  (EventDispatchers|BindEventtoOnSpawnEnemyUnitFinished (delegate Custom|BeginPlay_SpawnEnemyUnitFinished)))

(fn ConstructionScript)

(fn Initialize
  (params (GameBoard :type BP%20Game%20Board%20Object%20Reference))
  (Variables|Default|SetGameBoard GameBoard)
  ;[0.2396 0.2035 0 0.5] 敵の数はとりあえず固定値
  (Default|AddPool (Variables|Default|GetAC_ActorPool) "/Game/CM41/Blueprints/Units/Enemy/BP_EnemyUnit.BP_EnemyUnit_C" 3))

(fn PlaceUnitonRandomFreeCell
  (params (TargetUnit :type BP%20Unit%20Object%20Reference))
  (bind (_cellindex _result) (Default|GetRandomFreeCell (Variables|Default|GetGameBoard)))
  (if _result
    (Default|PlaceUnitonCell (Variables|Default|GetGameBoard) TargetUnit _cellindex (Default|GetRandomDirection (Variables|Default|GetGameBoard)))
    (return TargetUnit)
    (else
      (Development|PrintString "SpawnEnemyUnit : No Free Cell!" true true "(R=1.000000,G=0.000000,B=0.000000,A=1.000000)" 1e+02))))

(fn RemoveDeadUnits
  (for _array_element (Variables|Default|GetActiveEnemyUnits)
    ;[0.15 0.15 0.15 0.5 14] 死亡がマークされていないUnitのみを残す
    (if (not (.bDead (Utilities|Struct|BreakF_EnemyUnitData _array_element)))
      (Utilities|Array|AddUnique (LocalVariables|GetWorkArray) _array_element)))
  ;[0.15 0.15 0.15 0.5 14] Unit配列を差し替え
  (Variables|Default|SetActiveEnemyUnits (LocalVariables|GetWorkArray))
  (return))

(fn DecideUnitCommands
  (Utilities|Array|Clear (Variables|Default|GetUnitCommands))
  (for _array_element (Variables|Default|GetActiveEnemyUnits)
    (if (and (.bStandby (Utilities|Struct|BreakF_EnemyUnitData _array_element)) (not (.bDead (Utilities|Struct|BreakF_EnemyUnitData _array_element))))
      (bind _asbp_enemy_unit_controller (Utilities|Casting|CastToBP_EnemyUnitController (Pawn|GetController (.Unit (Utilities|Struct|BreakF_EnemyUnitData _array_element))))
        (:then
          (bind _unitcommand (Default|DecideUnitCommand _asbp_enemy_unit_controller self))
          (Utilities|Array|AddUnique (Variables|Default|GetUnitCommands) _unitcommand))
        (:CastFailed
          (Development|PrintString "BuildUnitCommands: Controller cast failed for EnemyUnit!" true true "(R=0.239583,G=0.035563,B=0.053270,A=0.500000)" 1e+02)))))
  (return))