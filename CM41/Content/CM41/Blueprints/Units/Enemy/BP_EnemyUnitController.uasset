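; AI controller for an enemy unit on the grid game board, choosing its next command.
; DecideUnitCommand builds an attack command against the first adjacent player unit found, otherwise a move to a random free adjacent cell, or nothing if boxed in.
; Position and death handlers keep the GameBoard's unit-cell map current, and death is also broadcast.
; Assumes a BP_GameBoard is already placed in the level.
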(event EventBeginPlay
  ;[0.15 0.15 0.15 0.5 14] Level 上に GameBoard が配置済であること前提
  (bind _returnvalue (Actor|GetActorOfClass "/Game/CM41/Blueprints/GameBoard/BP_GameBoard.BP_GameBoard_C"))
  (Variables|Default|SetGameBoard _returnvalue))

(event EventPossess
  (params (PossessedPawn :type Pawn%20Object%20Reference))
  (bind _asbp_unit (Utilities|Casting|CastToBP_Unit PossessedPawn))
  (Variables|Default|SetControlledUnit _asbp_unit))

(event EventUnPossess
  (params (UnpossessedPawn :type Pawn%20Object%20Reference))
  (Variables|Default|SetControlledUnit 0))

(event EventHandlePositionChanged
  (params (Unit :type BP%20Unit%20Object%20Reference) (From :type Int%20Point%20Structure) (To :type Int%20Point%20Structure))
  (Default|UpdateUnitCellRelations (Variables|Default|GetGameBoard) Unit From To))

(event EventHandleDeathFinished
  (params (Unit :type BP%20Unit%20Object%20Reference))
  (Default|RemoveUnitCellRelations (Variables|Default|GetGameBoard) Unit)
  (Default|CallOnEnemyUnitDeathFinished self Unit))

(fn ConstructionScript)

(fn DecideUnitCommand
  (params (CommandOuter :type Actor%20Object%20Reference))
  ;[0.15 0.15 0.15 0.5 14] この Unit の隣接セルに PlayerUnit が居るかチェック ＆ 取得
  (bind (_hitresult _hitcellindex) (CallFunction|FindAdjacentPlayerUnitCell (Variables|/Game/CM41/Blueprints/Units/BP_Unit.BP_Unit_C|GetCellIndex (Variables|Default|GetControlledUnit))))
  (if _hitresult
    ;[0.15 0.15 0.15 0.5 14] 隣接タイルにプレイヤーが居たら攻撃
    (bind _command (CallFunction|CreateCommandAttack _hitcellindex))
    (return _command)
    (else
      ;[0.15 0.15 0.15 0.5 14] 空いている隣接タイルへランダムに移動
      (bind _result (Default|GetAdjacentFreeCells (Variables|Default|GetGameBoard) (Variables|/Game/CM41/Blueprints/Units/BP_Unit.BP_Unit_C|GetCellIndex (Variables|Default|GetControlledUnit))))
      (if (not (== (.OutIndex (Utilities|Array|Random _result)) -1))
        (bind _command_2 (CallFunction|CreateCommandMove (.OutItem (Utilities|Array|Random _result))))
        (return _command_2)
        (else
          ;[0.15 0.15 0.15 0.5] 何も出来ない時
          (return 0))))))

(fn FindAdjacentPlayerUnitCell
  (params (CenterCellIndex :type Int%20Point%20Structure))
  (bind _result (Default|GetAdjacentCells (Variables|/Game/CM41/Blueprints/GameBoard/BP_GameBoard.BP_GameBoard_C|GetAC_Grid (Variables|Default|GetGameBoard)) CenterCellIndex))
  (bind _array_element (Utilities|Array|ForEachLoopwithBreak _result :!label _label)
    (:LoopBody
      (bind _output_get (LocalVariables|SetCurrentUnit (.Value (Utilities|Map|Find (Variables|/Game/CM41/Blueprints/GameBoard/BP_GameBoard.BP_GameBoard_C|GetCellUnitMap (Variables|Default|GetGameBoard)) _array_element))))
      (if (and (Class|GameplayStatics|ObjectIsA _output_get "/Game/CM41/Blueprints/Units/Player/BP_PlayerUnit.BP_PlayerUnit_C") (.ReturnValue (Utilities|Map|Find (Variables|/Game/CM41/Blueprints/GameBoard/BP_GameBoard.BP_GameBoard_C|GetCellUnitMap (Variables|Default|GetGameBoard)) _array_element)))
        (LocalVariables|SetCellIndex (Variables|/Game/CM41/Blueprints/Units/BP_Unit.BP_Unit_C|GetCellIndex (LocalVariables|GetCurrentUnit)))
        (LocalVariables|SetbHit true)
        (goto _label Break)))
    (:Completed
      (return (LocalVariables|GetbHit) (LocalVariables|GetCellIndex)))))

(fn CreateCommandMove
  (params (ToCellIndex :type Int%20Point%20Structure))
  (bind _returnvalue (Game|ConstructObjectfromClass "/Game/CM41/Blueprints/Units/BP_UnitCommand_Move.BP_UnitCommand_Move_C"))
  (bind _command (Default|SetParams _returnvalue (Variables|Default|GetControlledUnit) ToCellIndex (Default|GetDirectionBetweenCells (Variables|/Game/CM41/Blueprints/GameBoard/BP_GameBoard.BP_GameBoard_C|GetAC_Grid (Variables|Default|GetGameBoard)) (Variables|/Game/CM41/Blueprints/Units/BP_Unit.BP_Unit_C|GetCellIndex (Variables|Default|GetControlledUnit)) ToCellIndex) (Default|GetCellRelativeLocation (Variables|/Game/CM41/Blueprints/GameBoard/BP_GameBoard.BP_GameBoard_C|GetAC_Grid (Variables|Default|GetGameBoard)) ToCellIndex)))
  (return _command))

(fn CreateCommandAttack
  (params (ToCellIndex :type Int%20Point%20Structure))
  (bind _returnvalue (Game|ConstructObjectfromClass "/Game/CM41/Blueprints/Units/BP_UnitCommand_Attack.BP_UnitCommand_Attack_C"))
  (bind _command (Default|SetParams _returnvalue (Variables|Default|GetControlledUnit) ToCellIndex (Default|GetDirectionBetweenCells (Variables|/Game/CM41/Blueprints/GameBoard/BP_GameBoard.BP_GameBoard_C|GetAC_Grid (Variables|Default|GetGameBoard)) (Variables|/Game/CM41/Blueprints/Units/BP_Unit.BP_Unit_C|GetCellIndex (Variables|Default|GetControlledUnit)) ToCellIndex) (Default|GetCellRelativeLocation (Variables|/Game/CM41/Blueprints/GameBoard/BP_GameBoard.BP_GameBoard_C|GetAC_Grid (Variables|Default|GetGameBoard)) ToCellIndex) (.Value (Utilities|Map|Find (Variables|/Game/CM41/Blueprints/GameBoard/BP_GameBoard.BP_GameBoard_C|GetCellUnitMap (Variables|Default|GetGameBoard)) ToCellIndex))))
  (return _command))