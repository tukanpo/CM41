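; Player controller for a turn-based grid game that drives the possessed BP_Unit on the level's BP_GameBoard.
; Move, rotate and attack inputs are accepted only while the unit is idle with action points left, with directions snapped to four ways.
; Each becomes an executed command object; moves update board occupancy first, or become rotations if the cell isn't free.
; When a command finishes with no action points left, it signals turn end.
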(event EventBeginPlay
  (Utilities|FlowControl|Sequence
    (:then_0
      ;[0.15 0.15 0.15 0.5 14] Level 上に GameBoard が配置済であること前提
      (bind _returnvalue (Actor|GetActorOfClass "/Game/CM41/Blueprints/GameBoard/BP_GameBoard.BP_GameBoard_C"))
      (Variables|Default|SetGameBoard _returnvalue)
      (Input|AddMappingContext (PlayerController|LocalPlayerSubsystems|GetEnhancedInputLocalPlayerSubsystem) "/Game/CM41/Input/IMC_InGame.IMC_InGame" 0 "(bIgnoreAllPressedKeysUntilRelease=True,bForceImmediately=False,bNotifyUserSettings=False)"))))

(event EventPossess
  (params (PossessedPawn :type Pawn%20Object%20Reference))
  (bind _asbp_unit (Utilities|Casting|CastToBP_Unit PossessedPawn))
  (Variables|Default|SetControlledUnit _asbp_unit))

(event EventUnPossess
  (params (UnpossessedPawn :type Pawn%20Object%20Reference))
  (Variables|Default|SetControlledUnit 0) ; 空にする
)

(event Custom|ExecuteCommand_CommandFinished
  (EventDispatchers|UnbindEventfromOnCommandFinished (stale Custom|ExecuteCommand Command) (delegate Custom|ExecuteCommand_CommandFinished))
  (CallFunction|HandleUnitCommandFinished))

(event Custom|ExecuteCommand
  (params (Command :type BP%20Unit%20Command%20Object%20Reference))
  (EventDispatchers|BindEventtoOnCommandFinished Command (delegate Custom|ExecuteCommand_CommandFinished))
  (Default|Execute Command))

(event Input|EnhancedActionEvents|EnhancedInputActionIA_Move
  (params (ActionValue :type Vector%202D%20Structure) (ElapsedSeconds :type Float%20%28double-precision%29) (TriggeredSeconds :type Float%20%28double-precision%29) (InputAction :type Input%20Action%20Object%20Reference :default "/Game/CM41/Input/IA_Move.IA_Move"))
  (Utilities|CanAcceptInputMacro
    (:True
      (bind _command (CallFunction|ProcessInputMove ActionValue))
      (CallFunction|ExecuteCommand _command))))

(event Input|EnhancedActionEvents|EnhancedInputActionIA_Rotate
  (params (ActionValue :type Vector%202D%20Structure) (ElapsedSeconds :type Float%20%28double-precision%29) (TriggeredSeconds :type Float%20%28double-precision%29) (InputAction :type Input%20Action%20Object%20Reference :default "/Game/CM41/Input/IA_Rotate.IA_Rotate"))
  (Utilities|CanAcceptInputMacro
    (:True
      (bind _command (CallFunction|ProcessInputRotate ActionValue))
      (CallFunction|ExecuteCommand _command))))

(event Input|EnhancedActionEvents|EnhancedInputActionIA_Attack
  (params (ActionValue :type Boolean) (ElapsedSeconds :type Float%20%28double-precision%29) (TriggeredSeconds :type Float%20%28double-precision%29) (InputAction :type Input%20Action%20Object%20Reference :default "/Game/CM41/Input/IA_Attack.IA_Attack"))
  (Utilities|CanAcceptInputMacro
    (:True
      (bind _command (CallFunction|ProcessInputAttack))
      (CallFunction|ExecuteCommand _command))))

(event Input|KeyboardEvents|Escape
  (params (Key :type Key%20Structure :default "None"))
  (:Pressed
    (Game|QuitGame 0 "Quit" false)))

(fn ConstructionScript)

(fn SnapVector2DtoCardinal
  (params (InVec :type Vector%202D%20Structure))
  (bind (_x _y) (Math|Vector2D|BreakVector2D InVec))
  (bind (_x_2 _y_2) (Math|Vector2D|BreakVector2D InVec))
  (if (> (Math|Float|Absolute(Float) _x) (Math|Float|Absolute(Float) _y))
    (return (Utilities|Struct|MakeIntPoint (Math|Float|Truncate (Math|Float|Sign(Float) _x_2)) 0))
    (else
      (return (Utilities|Struct|MakeIntPoint 0 (Math|Float|Truncate (Math|Float|Sign(Float) _y_2)))))))

(fn CanAcceptInput
  (Utilities|IsValid (Variables|Default|GetControlledUnit)
    (:Is%20Valid
      ;[0.2396 0.2035 0 0.5 14] とりあえず IdleState のみ入力許可
      (if (Class|GameplayStatics|ObjectIsA (Variables|/Game/CM41/Blueprints/Common/StateMachine/AC_StateMachine.AC_StateMachine_C|GetCurrentState (Variables|/Game/CM41/Blueprints/Units/BP_Unit.BP_Unit_C|GetAC_UnitSM (Variables|Default|GetControlledUnit))) "/Game/CM41/Blueprints/Units/AC_UnitSM_IdleState.AC_UnitSM_IdleState_C")
        ;[0.15 0.15 0.15 0.5 14] 残APチェック
        (if (> (Variables|/Game/CM41/Blueprints/Units/BP_Unit.BP_Unit_C|GetActionPoint (Variables|Default|GetControlledUnit)) 0)
          (return true)
          (else
            (return false)))
        (else
          (return false))))
    (:Is%20Not%20Valid
      (return false))))

(fn ConvertInputVector2DtoMoveInfo
  (params (ActionValue :type Vector%202D%20Structure))
  (bind _result (CallFunction|SnapVector2DtoCardinal ActionValue))
  (bind _direction (Default|GetDirectionbyDeltaIndex (Variables|/Game/CM41/Blueprints/GameBoard/BP_GameBoard.BP_GameBoard_C|GetAC_Grid (Variables|Default|GetGameBoard)) _result))
  (return _result _direction))

(fn HandleUnitCommandFinished
  (if (<= (Variables|/Game/CM41/Blueprints/Units/BP_Unit.BP_Unit_C|GetActionPoint (Variables|Default|GetControlledUnit)) 0)
    (Default|CallOnPlayerTurnEnd)
    (return)))

(fn ProcessInputMove
  (params (ActionValue :type Vector%202D%20Structure))
  ;[0.15 0.15 0.15 0.5 14] 入力値を４方向にスナップして方向とオフセットを算出
  (bind (_celloffset _direction) (CallFunction|ConvertInputVector2DtoMoveInfo ActionValue))
  (LocalVariables|SetNewDirection _direction)
  ;[0.15 0.15 0.15 0.5 14] ４方向の入力値をセル座標のオフセット値として扱い、
  ; 現在位置にオフセット先を加算した CellIndex を取得。
  ; これが移動先のセル座標となる。
  (LocalVariables|SetNewCellIndex (+ (Variables|/Game/CM41/Blueprints/Units/BP_Unit.BP_Unit_C|GetCellIndex (Variables|Default|GetControlledUnit)) _celloffset))
  ;[0.15 0.15 0.15 0.5 14] FreeCell かチェック
  (if (Utilities|Set|Contains (Variables|/Game/CM41/Blueprints/GameBoard/BP_GameBoard.BP_GameBoard_C|GetFreeCells (Variables|Default|GetGameBoard)) (LocalVariables|GetNewCellIndex))
    ;[0.15 0.15 0.15 0.5 14] 移動コマンド発行 と実行
    ;;[0.2396 0.2035 0 0.5 14] Unit / Cell の参照情報を更新
    (Default|UpdateUnitCellRelations (Variables|Default|GetGameBoard) (Variables|Default|GetControlledUnit) (LocalVariables|GetNewCellIndex))
    (bind _returnvalue (Game|ConstructObjectfromClass "/Game/CM41/Blueprints/Units/BP_UnitCommand_Move.BP_UnitCommand_Move_C"))
    (bind _command (Default|SetParams _returnvalue (Variables|Default|GetControlledUnit) (LocalVariables|GetNewCellIndex) (LocalVariables|GetNewDirection) (Default|GetCellRelativeLocation (Variables|/Game/CM41/Blueprints/GameBoard/BP_GameBoard.BP_GameBoard_C|GetAC_Grid (Variables|Default|GetGameBoard)) (LocalVariables|GetNewCellIndex))))
    (return _command)
    (else
      ;[0.15 0.15 0.15 0.5 14] 振り向きコマンド発行 と実行
      (bind _returnvalue_2 (Game|ConstructObjectfromClass "/Game/CM41/Blueprints/Units/BP_UnitCommand_Rotate.BP_UnitCommand_Rotate_C"))
      (bind _command_2 (Default|SetParams _returnvalue_2 (Variables|Default|GetControlledUnit) (LocalVariables|GetNewDirection)))
      (return _command_2))))

(fn ProcessInputRotate
  (params (ActionValue :type Vector%202D%20Structure))
  (bind _direction (CallFunction|ConvertInputVector2DtoMoveInfo ActionValue))
  ;[0.15 0.15 0.15 0.5 14] 振り向きコマンド発行
  (bind _returnvalue (Game|ConstructObjectfromClass "/Game/CM41/Blueprints/Units/BP_UnitCommand_Rotate.BP_UnitCommand_Rotate_C"))
  (bind _command (Default|SetParams _returnvalue (Variables|Default|GetControlledUnit) _direction))
  (return _command))

(fn ProcessInputAttack
  ;[0.15 0.15 0.15 0.5 14] 向いてる方向の１つ前の CellIndex を取得
  (bind _celloffset (Default|DirectiontoCellOffset (Variables|/Game/CM41/Blueprints/GameBoard/BP_GameBoard.BP_GameBoard_C|GetAC_Grid (Variables|Default|GetGameBoard)) (Variables|/Game/CM41/Blueprints/Units/BP_Unit.BP_Unit_C|GetDirection (Variables|Default|GetControlledUnit))))
  (LocalVariables|SetTargetCellIndex (+ _celloffset (Variables|/Game/CM41/Blueprints/Units/BP_Unit.BP_Unit_C|GetCellIndex (Variables|Default|GetControlledUnit))))
  ;[0.15 0.15 0.15 0.5 14] 攻撃する
  (bind _returnvalue (Game|ConstructObjectfromClass "/Game/CM41/Blueprints/Units/BP_UnitCommand_Attack.BP_UnitCommand_Attack_C"))
  (bind _command (Default|SetParams _returnvalue (Variables|Default|GetControlledUnit) (LocalVariables|GetTargetCellIndex) (Variables|/Game/CM41/Blueprints/Units/BP_Unit.BP_Unit_C|GetDirection (Variables|Default|GetControlledUnit)) (Default|GetCellRelativeLocation (Variables|/Game/CM41/Blueprints/GameBoard/BP_GameBoard.BP_GameBoard_C|GetAC_Grid (Variables|Default|GetGameBoard)) (LocalVariables|GetTargetCellIndex))))
  (return _command))