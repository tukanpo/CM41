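; Unit command that moves a unit to a new cell index, direction and relative location.
; SetParams stores the unit and target values and returns itself for chaining.
; Execute binds to the unit state machine's action-finished event before requesting ChangeMoveState, manually invoking the completion path if that request fails.
; Completion unbinds the handler and signals that the command has finished, regardless of result.
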(event Custom|Execute_UnitActionCompleted
  (params (Unit :type BP%20Unit%20Object%20Reference) (bResult :type Boolean))
  (EventDispatchers|UnbindEventfromOnUnitActionFinished (Variables|/Game/CM41/Blueprints/Units/BP_Unit.BP_Unit_C|GetAC_UnitSM (Variables|Default|GetUnit)) (delegate Custom|Execute_UnitActionCompleted))
  (Default|CallOnCommandFinished))

(event EventExecute
  (EventDispatchers|BindEventtoOnUnitActionFinished (Variables|/Game/CM41/Blueprints/Units/BP_Unit.BP_Unit_C|GetAC_UnitSM (Variables|Default|GetUnit)) (delegate Custom|Execute_UnitActionCompleted))
  (bind _result (Default|ChangeMoveState (Variables|Default|GetUnit) (Variables|Default|GetNewCellIndex) (Variables|Default|GetNewDirection) (Variables|Default|GetNewRelativeLocation)))
  (if (not _result)
    (CallFunction|ExecuteUnitActionCompleted (Variables|Default|GetUnit) false) ; 実行失敗時の時に呼ぶ
  ))

(fn SetParams
  (params (Unit :type BP%20Unit%20Object%20Reference) (NewCellIndex :type Int%20Point%20Structure) (NewDirection :type E_GridDirection%20Enum :default "NewEnumerator0") (NewRelativeLocation :type Vector))
  (Variables|Default|SetUnit Unit)
  (Variables|Default|SetNewCellIndex NewCellIndex)
  (Variables|Default|SetNewDirection NewDirection)
  (Variables|Default|SetNewRelativeLocation NewRelativeLocation)
  (return self))