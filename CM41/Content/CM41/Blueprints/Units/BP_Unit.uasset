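; BP_Unit is a grid-based unit actor with a cell index, N/S/E/W facing, action points and pooling-style activate/deactivate that hides and resets it.
; A component state machine starts in Idle and takes parameters for Move, Rotate and Attack states.
; Timed events animate movement, rotation and attack, then signal completion.
; Cell changes notify the controller through BPI_UnitEventHandler, and a work-in-progress lunge helper applies placeholder damage.
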(event Custom|RotateToDirection
  (params (Direction :type E_GridDirection%20Enum :default "NewEnumerator0") (OverTime :type Float%20%28double-precision%29))
  (bind _yaw (CallFunction|GetYawfromDirection Direction))
  (Components|MoveComponentTo (Variables|Transformation|GetRootComponent) (Transformation|GetActorLocation) (Math|Rotator|MakeRotator 0.0 0.0 _yaw) true true OverTime false)
  (Default|CallOnRotatetoDirectionFinished))

(event Custom|SimpleMove
  (params (RelativeLocation :type Vector) (OverTime :type Float%20%28double-precision%29))
  (Variables|Default|SetAnimState "NewEnumerator1")
  (Components|MoveComponentTo (Variables|Transformation|GetRootComponent) RelativeLocation (Transformation|GetActorRotation) true false OverTime false)
  (Utilities|FlowControl|Delay 0.1)
  (Default|CallOnSimpleMoveFinished))

(event Custom|SimpleAttack
  (Variables|Default|SetAnimState "NewEnumerator4")
  ;[0.2396 0.2035 0 0.5] 要キャンセル対応
  (Utilities|FlowControl|Delay 0.833333)
  (Default|CallOnSimpleAttackFinished))

(event EventBeginPlay
  ;[0.15 0.15 0.15 0.5 14] Unit ステートマシンの初期化と実行
  (Default|Initialize (Variables|Default|GetAC_UnitSM) "/Game/CM41/Blueprints/Units/AC_UnitSM_State.AC_UnitSM_State_C")
  (Default|ChangeState (Variables|Default|GetAC_UnitSM) "/Game/CM41/Blueprints/Units/AC_UnitSM_IdleState.AC_UnitSM_IdleState_C"))

(fn ConstructionScript)

(fn ActivateInternal
  (Variables|Default|SetbActive true)
  (Rendering|SetActorHiddenInGame false)
  (Collision|SetActorEnableCollision true)
  (Actor|Tick|SetActorTickEnabled true)
  (return))

(fn DeactivateInternal
  (Variables|Default|SetbActive false)
  (Rendering|SetActorHiddenInGame true)
  (Collision|SetActorEnableCollision false)
  (Actor|Tick|SetActorTickEnabled false)
  (CallFunction|ResetStatus)
  (return))

(fn ResetStatus
  ;[0.15 0.15 0.15 0.5 14] 変数等を初期化
  (Transformation|SetActorLocationAndRotation "0, 0, 0" "0, 0, 0")
  (Variables|Default|SetCellIndex (Utilities|Struct|MakeIntPoint -1 -1))
  (Variables|Default|SetDirection "NewEnumerator0")
  (Variables|Default|SetAnimState "NewEnumerator0"))

(fn ChangeDirection
  (params (NewDirection :type E_GridDirection%20Enum :default "NewEnumerator0"))
  ;[0.15 0.15 0.15 0.5 14] Direction に応じて Unit の向きを瞬時に変える
  (Transformation|SetActorRotation (Math|Rotator|MakeRotator 0.0 0.0 (Utilities|Select :Index NewDirection :NewEnumerator0 0.0 :NewEnumerator1 1.8e+02 :NewEnumerator2 9e+01 :NewEnumerator3 -9e+01)))
  ;[0.15 0.15 0.15 0.5 14] 保持している向きも更新
  (Variables|Default|SetDirection NewDirection)
  (return))

(fn SetLocationandDirection
  (params (WorldLocation :type Vector) (Direction :type E_GridDirection%20Enum :default "NewEnumerator0"))
  (Transformation|SetActorTransform (Math|Conversions|ToTransform(Vector) WorldLocation))
  (CallFunction|ChangeDirection Direction))

(fn GetYawfromDirection
  (params (Direction :type E_GridDirection%20Enum :default "NewEnumerator0"))
  (switch Utilities|FlowControl|Switch|SwitchonE_GridDirection Direction
    (:NewEnumerator0
      (return 0.0))
    (:NewEnumerator1
      (return 1.8e+02))
    (:NewEnumerator2
      (return 9e+01))
    (:NewEnumerator3
      (return 2.7e+02))))

(fn GetVectorbyDirection
  (params (Direction :type E_GridDirection%20Enum :default "NewEnumerator0"))
  (switch Utilities|FlowControl|Switch|SwitchonE_GridDirection Direction
    (:NewEnumerator0
      (return "1.000000,0.000000,0.000000"))
    (:NewEnumerator1
      (return "-1.000000,0.000000,0.000000"))
    (:NewEnumerator2
      (return "0.000000,1.000000,0.000000"))
    (:NewEnumerator3
      (return "0.000000,-1.000000,0.000000"))))

(fn ChangeCellIndex
  (params (NewCellIndex :type Int%20Point%20Structure))
  (Utilities|FlowControl|Sequence
    (:then_0
      (LocalVariables|SetPrevCellIndex (Variables|Default|GetCellIndex))
      (Variables|Default|SetCellIndex NewCellIndex))
    (:then_1
      (if (Utilities|DoesObjectImplementInterface (Pawn|GetController) "/Game/CM41/Blueprints/Units/BPI_UnitEventHandler.BPI_UnitEventHandler_C")
        (Class|BPIUnitEventHandler|HandlePositionChanged(Message) (Pawn|GetController) self (LocalVariables|GetPrevCellIndex) NewCellIndex)
        (return)
        (else
          (Development|PrintString "ChangeCellIndex: BPI_UnitEventHandler does not implemented!" true true "(R=0.239583,G=0.035563,B=0.053270,A=0.500000)" 1e+03)
          (return))))))

(fn ModifyActionPoint
  (params (Delta :type Integer))
  (bind _output_get (Variables|Default|SetActionPoint (+ Delta (Variables|Default|GetActionPoint))))
  (return _output_get))

(fn ChangeMoveState
  (params (NewCellIndex :type Int%20Point%20Structure) (NewDirection :type E_GridDirection%20Enum :default "NewEnumerator0") (NewRelativeLocation :type Vector))
  (Default|SetMoveParams (Variables|Default|GetAC_UnitSM_MoveState) NewCellIndex NewDirection NewRelativeLocation)
  (bind _bresult (Default|ChangeState (Variables|Default|GetAC_UnitSM) "/Game/CM41/Blueprints/Units/AC_UnitSM_MoveState.AC_UnitSM_MoveState_C"))
  (return _bresult))

(fn ChangeRotateState
  (params (NewDirection :type E_GridDirection%20Enum :default "NewEnumerator0"))
  (Default|SetParams (Variables|Default|GetAC_UnitSM_RotateState) NewDirection)
  (bind _bresult (Default|ChangeState (Variables|Default|GetAC_UnitSM) "/Game/CM41/Blueprints/Units/AC_UnitSM_RotateState.AC_UnitSM_RotateState_C"))
  (return _bresult))

(fn ChangeAttackState
  (params (NewCellIndex :type Int%20Point%20Structure) (NewDirection :type E_GridDirection%20Enum :default "NewEnumerator0") (NewRelativeLocation :type Vector))
  (Default|SetAttackParams (Variables|Default|GetAC_UnitSM_AttackState) NewCellIndex NewDirection NewRelativeLocation)
  (bind _bresult (Default|ChangeState (Variables|Default|GetAC_UnitSM) "/Game/CM41/Blueprints/Units/AC_UnitSM_AttackState.AC_UnitSM_AttackState_C"))
  (return _bresult))

(fn Activate
  (Protected|ActivateInternal)
  (return true))

(fn Deactive
  (Protected|DeactivateInternal)
  (return true))

(fn IsActive
  (return (Variables|Default|GetbActive)))