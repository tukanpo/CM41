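; BP_UnitCommand_Rotate is a unit command that turns a Unit to face a new direction, with both set through a chainable SetParams.
; Execute binds to the unit state machine's action-finished event, then requests the rotate state change, reporting a failed finish if that request is rejected.
; On finish, success or failure, it unbinds, fires its command-finished callback and tells the CommandHandler the command is done.
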(event Custom|Execute_UnitActionFinished
  (params (bResult :type Boolean))
  (EventDispatchers|UnbindEventfromOnUnitActionFinished (Variables|/Game/CM41/Blueprints/Units/BP_Unit.BP_Unit_C|GetAC_UnitSM (Variables|Default|GetUnit)) (delegate Custom|Execute_UnitActionFinished))
  (Default|CallOnCommandFinished)
  (Default|HandleCommandFinished (stale EventExecute CommandHandler)))

(event EventExecute
  (params (CommandHandler :type BPI%20Command%20Event%20Handler%20Interface))
  (EventDispatchers|BindEventtoOnUnitActionFinished (Variables|/Game/CM41/Blueprints/Units/BP_Unit.BP_Unit_C|GetAC_UnitSM (Variables|Default|GetUnit)) (delegate Custom|Execute_UnitActionFinished))
  (bind _bresult (Default|ChangeRotateState (Variables|Default|GetUnit) (Variables|Default|GetNewDirection)))
  (if (not _bresult)
    (CallFunction|ExecuteUnitActionFinished false)))

(fn SetParams
  (params (Unit :type BP%20Unit%20Object%20Reference) (NewDirection :type E_GridDirection%20Enum :default "NewEnumerator0"))
  (Variables|Default|SetUnit Unit)
  (Variables|Default|SetNewDirection NewDirection)
  (return self))