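; BP_GameBoard is the grid game board that tracks where units stand and plays the camera's intro animation.
; ACGrid supplies cells and coordinates, filled with checkered default tiles on one instanced static mesh, colored through per-instance custom data.
; A FreeCells set and CellUnitMap track occupancy, supporting unit placement and random or adjacent free-cell lookups.
; GameBoardCamera derives its intro path from grid center and size, then the board signals completion.
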(event Custom|PlayInAnimation
  (EventDispatchers|BindEventtoOninAnimationFinished (Variables|Default|GetGameBoardCamera) (delegate Custom|PlayInTransition_InAnimationFinished))
  (bind (_resultstartlocation _resulttargetlocation) (Default|GetinAnimationLocations (Variables|Default|GetGameBoardCamera) (Default|GetGridWorldCenter (Variables|Default|GetAC_Grid)) (Default|GetGridWorldSize (Variables|Default|GetAC_Grid)) (Variables|Default|GetCameraPitch)))
  (Default|PlayinAnimation (Variables|Default|GetGameBoardCamera) _resultstartlocation _resulttargetlocation))

(event Custom|PlayInTransition_InAnimationFinished
  (EventDispatchers|UnbindEventfromOninAnimationFinished (Variables|Default|GetGameBoardCamera) (delegate Custom|PlayInTransition_InAnimationFinished))
  (Default|CallOninAnimationFinished))

(event EventBeginPlay)

(event Collision|EventActorBeginOverlap
  (params (OtherActor :type Actor%20Object%20Reference)))

(event EventTick
  (params (DeltaSeconds :type Float%20%28single-precision%29)))

(fn ConstructionScript
  (bind _gridsize (Variables|Default|GetGridSize))
  (bind (_x _y) (Utilities|Struct|BreakIntPoint _gridsize))
  ;[0.15 0.15 0.15 0.5 14] グリッドを初期化
  (Default|Initialize (Variables|Default|GetAC_Grid) _x _y (Variables|Default|GetCellSize))
  ;[0.15 0.15 0.15 0.5 14] セルをデフォルトタイルで埋める
  (CallFunction|FillDefaultTiles))

(fn Initialize
  (params (GridSize :type Int%20Point%20Structure) (CellSize :type Float%20%28double-precision%29) (bFillDefaultTiles :type Boolean))
  (bind (_x _y) (Utilities|Struct|BreakIntPoint GridSize))
  ;[0.15 0.15 0.15 0.5 14] Grid 初期化
  (Default|Initialize (Variables|Default|GetAC_Grid) _x _y CellSize)
  ;[0.15 0.15 0.15 0.5 14] 必要に応じてダミータイルで埋める
  (if bFillDefaultTiles
    (CallFunction|FillDefaultTiles))
  ;[0.15 0.15 0.15 0.5 14] フリーセル座標配列を初期化
  (bind _keys (Utilities|Map|Keys (Variables|/Game/CM41/Blueprints/Common/Grid/AC_Grid.AC_Grid_C|GetCells (Variables|Default|GetAC_Grid))))
  (Utilities|Set|AddItems (Variables|Default|GetFreeCells) _keys)
  (return))

(fn FillDefaultTiles
  (Components|InstancedStaticMesh|ClearInstances (Variables|Default|GetInstancedStaticMesh))
  (bind _keys (Utilities|Map|Keys (Variables|/Game/CM41/Blueprints/Common/Grid/AC_Grid.AC_Grid_C|GetCells (Variables|Default|GetAC_Grid))))
  (for _array_element _keys
    (CallFunction|AddDefaultTiletoISM (Math|Conversions|ToTransform(Vector) (Default|GetCellWorldLocation (Variables|Default|GetAC_Grid) _array_element)) _array_element)))

(fn AddDefaultTiletoISM
  (params (Transform :type Transform) (CellIndex :type Int%20Point%20Structure))
  (bind _color (CallFunction|GetDefaultTileCheckeredColor CellIndex))
  (bind (_r _g _b) (Math|Color|BreakColor _color))
  (bind _returnvalue (Components|InstancedStaticMesh|AddInstance (Variables|Default|GetInstancedStaticMesh) Transform false))
  ;[0.15 0.15 0.15 0.5] インスタンス毎にマテリアルの色を変える。
  ; マテリアル側でベースカラーに R(index:0), G(index:1), B(index:2) の３つの PerInstanceCustomData を設定している。
  (Components|InstancedStaticMesh|SetCustomDataValue (Variables|Default|GetInstancedStaticMesh) _returnvalue 0 _r false)
  (Components|InstancedStaticMesh|SetCustomDataValue (Variables|Default|GetInstancedStaticMesh) _returnvalue 1 _g false)
  (Components|InstancedStaticMesh|SetCustomDataValue (Variables|Default|GetInstancedStaticMesh) _returnvalue 2 _b true))

(fn GetDefaultTileCheckeredColor
  (params (CellIndex :type Int%20Point%20Structure))
  (if (== (Math|Integer|%(Integer) (+ (.x CellIndex) (.y CellIndex)) 2) 0)
    (return (Variables|Default|GetDefaultTileColor1))
    (else
      (return (Variables|Default|GetDefaultTileColor2)))))

(fn GetRandomFreeCell
  (if (> (Utilities|Set|Length (Variables|Default|GetFreeCells)) 0)
    (bind _result (Utilities|Set|ToArray (Variables|Default|GetFreeCells)))
    (return (.OutItem (Utilities|Array|Random _result)) true)
    (else
      (return "" false))))

(fn GetAdjacentFreeCells
  (params (CenterCellIndex :type Int%20Point%20Structure))
  (bind _enumvalue (|ForEachE_GridDirection)
    (:LoopBody
      (bind _result (Default|GetCellOffsetbyDirection (Variables|Default|GetAC_Grid) _enumvalue))
      (LocalVariables|SetWorkCellIndex (+ _result CenterCellIndex))
      (if (and (Default|IsinGridBounds (Variables|Default|GetAC_Grid) (LocalVariables|GetWorkCellIndex)) (Utilities|Set|Contains (Variables|Default|GetFreeCells) (LocalVariables|GetWorkCellIndex)))
        (Utilities|Array|AddUnique (LocalVariables|GetWorkCells) (LocalVariables|GetWorkCellIndex))))
    (:then
      (return (LocalVariables|GetWorkCells)))))

(fn PlaceUnitonCell
  (params (TargetUnit :type BP%20Unit%20Object%20Reference) (CellIndex :type Int%20Point%20Structure) (Direction :type E_GridDirection%20Enum :default "NewEnumerator0"))
  ;[0.15 0.15 0.15 0.5 14] Location と向きを設定
  (Default|SetLocationandDirection TargetUnit (Default|GetCellWorldLocation (Variables|Default|GetAC_Grid) CellIndex) Direction)
  (Default|ChangeCellIndex TargetUnit CellIndex)
  (return))

(fn GetRandomDirection
  (return (Utilities|Enum|ByteToEnumE_GridDirection (Math|Conversions|ToByte(Integer) (Math|Random|RandomIntegerinRange 0 (- (|GetNumEnumEntries) 1))))))

(fn UpdateUnitCellRelations
  (params (Unit :type BP%20Unit%20Object%20Reference) (PrevCellIndex :type Int%20Point%20Structure) (NextCellIndex :type Int%20Point%20Structure))
  (Utilities|FlowControl|Sequence
    (:then_0
      ;[0.15 0.15 0.15 0.5 14] 前のセル情報を消してフリーセルに追記
      (if (== (.Value (Utilities|Map|Find (Variables|Default|GetCellUnitMap) PrevCellIndex)) Unit)
        (Utilities|Map|Remove (Variables|Default|GetCellUnitMap) PrevCellIndex)
        (Utilities|Set|Add (Variables|Default|GetFreeCells) PrevCellIndex)))
    (:then_1
      ;[0.15 0.15 0.15 0.5 14] 次のセル情報を追加してフリーセルから除く
      (Utilities|Map|Add (Variables|Default|GetCellUnitMap) NextCellIndex Unit)
      (Utilities|Set|Remove (Variables|Default|GetFreeCells) NextCellIndex)
      (return))))

(fn RemoveUnitCellRelations
  (params (Unit :type BP%20Unit%20Object%20Reference))
  (Utilities|Map|Remove (Variables|Default|GetCellUnitMap) (Variables|/Game/CM41/Blueprints/Units/BP_Unit.BP_Unit_C|GetCellIndex Unit))
  (Utilities|Set|Add (Variables|Default|GetFreeCells) (Variables|/Game/CM41/Blueprints/Units/BP_Unit.BP_Unit_C|GetCellIndex Unit))
  ;[0.15 0.15 0.15 0.5 14] とりあえず -1 突っ込んでおく
  (Variables|/Game/CM41/Blueprints/Units/BP_Unit.BP_Unit_C|SetCellIndex Unit (Utilities|Struct|MakeIntPoint -1 -1))
  (return))